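; Base enemy character Blueprint that handles spawn-in and death presentation.
; On BeginPlay it reverses a timeline to animate dissolve and plays a random entry montage.
; Death immediately disables crowd avoidance; after the animation it freezes, drops capsule collision, removes UI and async-loads a color-matched Niagara effect.
; A shared SetDissolve drives body and weapon materials, and the death timeline destroys weapon, then character.
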(event `self.ReceiveBeginPlay`
  (bind _entrymontagestoplay (`self.EntryMontagesToPlay`))
  (`|ExecutionSequence`
    (:`then_0`
      ;[1 1 1] 敌人进场Montage动画和特效。
      (`TimelineComponent.SetPlayRate` (`self.EntryRestoreTimeline`) (/ 1.0 (`self.TotalEnteyRestoreTime`)))
      (bind (_direction _normalizedfloattrack) (`Timeline|EntryRestoreTimeline` :!via `ReverseFromEnd`)
        (:`Update`
          (`self.Set Dissolve` _normalizedfloattrack) ; 设置溶解效果。
        )))
    (:`then_1`
      (if (`KismetArrayLibrary.Array_IsNotEmpty` _entrymontagestoplay)
        (`self.PlayAnimMontage` (`KismetArrayLibrary.Array_Random` _entrymontagestoplay))))))

(event `/Game/EnemyCharacter/BPI_EnemyDeath.OnEnemyDiedImmediately `
  ;[1 1 1] 死亡后立刻关闭人群避障组件。否则播放动画时的移动也会对其他角色的避障计算造成影响。比如死亡的小兵飞向Boss时，Boss为了避开会进行奇怪的转身行为。
  (`WarriorAIController.SetCrowdComponentDeactivate` (`self.WarriorAIController`))
  (`KismetSystemLibrary.PrintString` "1111111"))

(event `/Game/EnemyCharacter/BPI_EnemyDeath.OnEnemyDiedAfterAnim`
  (params (DissolveNiagaraSystem :type "NiagaraSystem Soft Object Reference"))
  (bind _mesh (`self.Mesh`))
  (bind _returnvalue (`PawnCombatComponent.GetCharacterCurrentEquippedWeapon` (`self.EnemyCombatComponent`)))
  (`|ExecutionSequence`
    (:`then_0`
      ;[1 1 1] 停止动画，关闭碰撞器。
      (set `SkeletalMeshComponent.bPauseAnims` true (`self.Mesh`))
      (`PrimitiveComponent.SetCollisionEnabled` (`self.CapsuleComponent`) "NoCollision"))
    (:`then_1`
      ;[1 1 1] 移除敌人相关UI。
      (`EnemyUIComponent.RemoveEnemyDrawnWidgetsIfAny` (`self.EnemyUIComponent`)))
    (:`then_2`
      ;[1 1 1] 死亡特效FX。
      ;;[1 1 1] 创建并使用Niagara粒子特效。异步加载。
      (bind _object (`|LoadAsset` DissolveNiagaraSystem)
        (:`Completed`
          (bind _asniagara_system (cast `NiagaraSystem` _object))
          (bind _returnvalue_2 (`NiagaraFunctionLibrary.SpawnSystemAttached` _asniagara_system (`self.Mesh`) "None" (0.0 0.0 0.0) (struct) "KeepRelativeOffset" true))
          ;;;[1 1 1] 将材质消融颜色给到粒子特效。保持视觉效果一致。
          (bind _returnvalue_3 (`PrimitiveComponent.CreateDynamicMaterialInstance` _mesh 0 (`PrimitiveComponent.GetMaterial` _mesh 0) "None"))
          (bind _returnvalue_4 (`MaterialInstanceDynamic.K2_GetVectorParameterValue` _returnvalue_3 "DissolveEdgeColor"))
          (`NiagaraComponent.SetNiagaraVariableLinearColor` _returnvalue_2 "DissolveParticleColor" _returnvalue_4)
          ;;[1 1 1] 角色和武器消融效果。
          (`TimelineComponent.SetPlayRate` (`self.DissolveTimeline`) (/ 1.0 (`self.TotalDissolveTime`)))
          (bind (_direction _normalizedfloattrack) (`Timeline|DissolveTimeline` :!via `PlayFromStart`)
            (:`Update`
              (`self.Set Dissolve` _normalizedfloattrack) ; 设置溶解效果。
            )
            (:`Finished`
              ;;;[1 1 1] 先销毁武器，因为我们需要通过角色Actor上的Combat组件获取当前武器。
              (`/Engine/EditorBlueprintResources/StandardMacros.IsValid` _returnvalue
                (:`Is Valid`
                  (`self.K2_DestroyActor` _returnvalue))
                (:`Is Not Valid`
                  _))
              ;;;[1 1 1] 销毁自身角色。
              (`self.K2_DestroyActor`))))))))

(fn `Set Dissolve`
  (params (ParameterValue :type "Float (single-precision)"))
  (bind _returnvalue (`PawnCombatComponent.GetCharacterCurrentEquippedWeapon` (`self.EnemyCombatComponent`)))
  (`MeshComponent.SetScalarParameterValueOnMaterials` (`self.Mesh`) "DissolveAmount" ParameterValue)
  (`/Engine/EditorBlueprintResources/StandardMacros.IsValid` _returnvalue
    (:`Is Valid`
      (`MeshComponent.SetScalarParameterValueOnMaterials` (`WarriorWeaponBase.WeaponMesh` _returnvalue) "DissolveAmount" ParameterValue))))

(fn `UserConstructionScript`)