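; Survival game mode Blueprint that presents wave-based combat through UI and starts boss battle music on BeginPlay.
; It reacts to inherited survival state changes with wave announcements, countdowns and a time-limit widget that flags danger when timeout is critical.
; The last wave gets an extra notice and a spawn delay.
; Victory or failure clears widgets, fades the camera and async-loads the win or lose screen, with failure also tagging the player dead.
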(event `self.ReceiveBeginPlay`
  (`|ExecutionSequence`
    (:`then_0`
      (`GameplayStatics.SpawnSound2D` "/Game/Assets/Sounds/Music/Dungeons_EndBossBattle.Dungeons_EndBossBattle" 1.0 1.0 0.0 null))
    (:`then_1`
      (add `self.OnSurvivalGameModeStateChanged` (delegate `OnSurvivalGameModeStateChanged_Event`)))))

(event `OnSurvivalGameModeStateChanged_Event` :!signature `self.OnSurvivalGameModeStateChanged`
  (params (CurrentState :type "EWarriorSurvivalGameModeState Enum" :default "WaitSpawnNewWave"))
  (bind _wbp_wavelimittime (`self.WBP_WaveLimitTime`))
  (switch `EWarriorSurvivalGameModeState` CurrentState
    (:`WaitSpawnNewWave`
      ;[1 1 1] Wait Spawn New Wave.
      (`self.CreateWidgetWaveCountDown` "New Wave Coming In" (`self.SpawnNewWaveWaitTime`)))
    (:`SpawningNewWave`
      ;[1 1 1] Spawning New Wave.
      (`self.CreateWidgetWave` (`|FormatText` "Wave {CurrentWaveCount}" (`self.CurrentWaveCount`)))
      ;;[1 1 1] 最后一波时，额外UI提示。
      (if (== (`self.CurrentWaveCount`) (`self.TotalWavesToSpawn`))
        (set `self.SpawnEnemiesDelayTime` 4.0)
        (`KismetSystemLibrary.Delay` 2.0)
        (`self.CreateWidgetWave` "Last Wave")))
    (:`BattleStarted`
      ;[1 1 1] BattleStarted
      (`|ExecutionSequence`
        (:`then_0`
          (`/Engine/EditorBlueprintResources/StandardMacros.IsValid` _wbp_wavelimittime
            (:`Is Not Valid`
              (bind _returnvalue (`|CreateWidget` "/Game/Widgets/GameModeWidgets/WBP_WaveLimitTime.WBP_WaveLimitTime_C"))
              (`UserWidget.AddToViewport` _returnvalue 0)
              (set `self.WBP_WaveLimitTime` _returnvalue))))
        (:`then_1`
          (`/Game/Widgets/GameModeWidgets/WBP_WaveLimitTime.StartLimitTime` _wbp_wavelimittime (`self.CurrentWaveLimitTime`) (or (not (`self.CurrentWhenWaveOverGoToNext`)) (and (`self.HasFinishedAllWaves`) (> (`self.CurrentWaveLimitTime`) 0.0)))))))
    (:`WaveCompleted`
      ;[1 1 1] Wave Completed or TimedOut.
      (`|ExecutionSequence` :!label _label
        (:`then_0`
          (bind _wbp_wavelimittime_2 (`self.WBP_WaveLimitTime`)
            (:`then`
              (`/Game/Widgets/GameModeWidgets/WBP_WaveLimitTime.CancelLimitTime` _wbp_wavelimittime_2))
            (:`else`)))
        (:`then_1`
          (if (not (`self.HasFinishedAllWaves`))
            (`self.CreateWidgetWaveCountDown` (`KismetMathLibrary.SelectText` (`|FormatText` "Wave {CurrentWaveCount} Completed" (`self.CurrentWaveCount`)) (`|FormatText` "Wave {CurrentWaveCount} Timed Out" (`self.CurrentWaveCount`)) (`|EnumEquality` (`self.CurrentSurvivalGameModeState`) "WaveCompleted")) (`self.WaveCompletedWaitTime`))))))
    (:`WaveTimedOut`
      (goto _label))
    (:`AllWavesDone`
      ;[1 1 1] 获胜UI。
      (`KismetSystemLibrary.Delay` 1.5)
      (`WidgetLayoutLibrary.RemoveAllWidgets`)
      (`PlayerCameraManager.StartCameraFade` :`self` (`GameplayStatics.GetPlayerCameraManager` 0) :`ToAlpha` 1.0 :`Duration` 3.0 :`bHoldWhenFinished` true)
      (`KismetSystemLibrary.Delay` 3.0)
      (bind _class (`|LoadAssetClass` "/Game/Widgets/Main/WBP_WinScreen.WBP_WinScreen_C")
        (:`Completed`
          (bind _asuser_widget (castclass `UserWidget` _class))
          (bind _returnvalue_2 (`|CreateWidget` _asuser_widget))
          (`UserWidget.AddToViewport` _returnvalue_2 0))))
    (:`Failed`
      ;[1 1 1] 失败UI。
      (`|ExecutionSequence`
        (:`then_0`
          (`WarriorFunctionLibrary.AddGameplayTagToActorIfNone` (`GameplayStatics.GetPlayerPawn` 0) (struct :`TagName` "Shared.Status.Dead")))
        (:`then_1`
          (`KismetSystemLibrary.Delay` 2.0)
          (`WidgetLayoutLibrary.RemoveAllWidgets`)
          (`PlayerCameraManager.StartCameraFade` :`self` (`GameplayStatics.GetPlayerCameraManager` 0) :`ToAlpha` 1.0 :`Duration` 2.0 :`bHoldWhenFinished` true)
          (`KismetSystemLibrary.Delay` 2.0)
          (bind _class_2 (`|LoadAssetClass` "/Game/Widgets/Main/WBP_LoseScreen.WBP_LoseScreen_C")
            (:`Completed`
              (bind _asuser_widget_2 (castclass `UserWidget` _class_2))
              (bind _returnvalue_3 (`|CreateWidget` _asuser_widget_2))
              (`UserWidget.AddToViewport` _returnvalue_3 0))))))))

(event `self.ReceiveDestroyed`)

(fn `CreateWidgetWave`
  (params (TextContentToDisplay :type Text))
  (bind _returnvalue (`|CreateWidget` "/Game/Widgets/GameModeWidgets/WBP_WaveText.WBP_WaveText_C"))
  (`UserWidget.AddToViewport` _returnvalue 0)
  (`/Game/Widgets/GameModeWidgets/WBP_WaveText.SetText` _returnvalue TextContentToDisplay))

(fn `CreateWidgetWaveCountDown`
  (params (TextContentToDisplay :type Text) (InTotalCountDownTime :type "Float (double-precision)"))
  (bind _returnvalue (`|CreateWidget` "/Game/Widgets/GameModeWidgets/WBP_WaveTextWithCountDown.WBP_WaveTextWithCountDown_C"))
  (`UserWidget.AddToViewport` _returnvalue 0)
  (`/Game/Widgets/GameModeWidgets/WBP_WaveTextWithCountDown.SetText` _returnvalue TextContentToDisplay)
  (`/Game/Widgets/GameModeWidgets/WBP_WaveTextWithCountDown.StartCountDown` _returnvalue InTotalCountDownTime))

(fn `UserConstructionScript`)