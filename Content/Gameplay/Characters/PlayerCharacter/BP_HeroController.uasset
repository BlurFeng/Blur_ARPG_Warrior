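; Hero player controller that tracks switches between keyboard/mouse and gamepad, intended to update on-screen control prompts.
; A countdown started on BeginPlay polls the UINav component repeatedly, even during pause, and calls OnInputHardwareChange on the first check or any change; Destroyed cancels it.
; Root widget add and remove events switch input between Game and UI and Game Only.
; Mouse cursor visibility logic is present but disconnected.
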(event `self.ReceiveBeginPlay`
  (`self.CheckInpudHardwareStart`))

(event `self.ReceiveDestroyed`
  (`self.CheckInpudHardwareCancel`))

(event `self.OnRootWidgetAdded`
  (`WidgetBlueprintLibrary.SetInputMode_GameAndUIEx` self null))

(event `self.OnRootWidgetRemoved`
  (`WidgetBlueprintLibrary.SetInputMode_GameOnly` self))

(event `CheckInpudHardwareStart`
  (bind _isusinggamepad (`self.IsUsingGamepad`))
  ;[1 1 1] 根据键鼠或手柄输入变化切换显示操作提示。
  (`WarriorFunctionLibrary.CountDown` -1.0 0.2 true false :!label _label
    (:`Update`
      (if (or (!= _isusinggamepad (`self.IsUsingGamepadCached`)) (`self.IsUsingGamepadCheckFirst`))
        (bind _output_get (set `self.IsUsingGamepadCached` _isusinggamepad))
        (set `self.IsUsingGamepadCheckFirst` false)
        (`|ExecutionSequence`
          (:`then_1`
            (`self.OnInputHardwareChange` _output_get)))))))

(event `CheckInpudHardwareCancel`
  ;[1 1 1] 根据键鼠或手柄输入变化切换显示操作提示。
  (goto _label :!via `Cancel`))

(fn `IsUsingGamepad`
  (returns (IsUsingGamepad :type Boolean))
  (return (`UINavPCComponent.IsUsingGamepad` (`self.UINavPC`))))

(fn `UserConstructionScript`)