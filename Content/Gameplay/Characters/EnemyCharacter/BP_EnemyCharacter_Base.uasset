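; Base enemy character Blueprint that handles entry, death and emissive status feedback.
; BeginPlay reverses a dissolve timeline alongside a random montage, holding an Entering gameplay tag briefly.
; Death disables crowd avoidance, then ragdolls, removes UI and async-loads color-matched Niagara while dissolving body and weapon, finally triggering the SpawnStone ability and destroying both.
; SetEmissiveFX uses countdown updates to lerp emissive color and intensity on mesh materials.
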(event `SetEmissiveFX`
  (params (Enable :type Boolean) (FXType :type Integer))
  ;[1 1 1] EmissiveFX角色发光特效。用来提示一些状态，比如受击或无敌。
  (`|ExecutionSequence`
    (:`then_0`
      (set `self.EmissiveFXSpeed` (select `int` FXType :`0` 0.4 :`1` 0.1 :!type "Float (single-precision)"))
      (`|ExecutionSequence`
        (:`then_0`
          (goto _label :!via `Cancel`))
        (:`then_1`
          (`WarriorFunctionLibrary.CountDown` -1.0 0.0 :!label _label
            (:`Update`
              (bind _completed (`self.LerpSetEmissiveFXColor` (select `int` FXType :`0` (struct :`R` 0.709804 :`G` 0.066667 :`A` 1.0) :`1` (struct :`R` 0.84375 :`G` 0.803642 :`B` 0.229458 :`A` 1.0) :!type "LinearColor Structure") (`self.EmissiveFXSpeed`)))
              (if _completed
                (goto _label :!via `Cancel`)))))))
    (:`then_1`
      (if Enable
        (`WarriorFunctionLibrary.CountDown` -1.0 0.0 :!label _label_2
          (:`Update`
            (bind _completed_2 (`self.LerpSetEmissiveFXValue` 1.0 (`self.EmissiveFXSpeed`)))
            (if _completed_2
              (goto _label_2 :!via `Cancel`))))
        (else
          (`|ExecutionSequence`
            (:`then_0`
              (goto _label_2 :!via `Cancel`))
            (:`then_1`
              (`WarriorFunctionLibrary.CountDown` -1.0 0.0 :!label _label_3
                (:`Update`
                  (bind _completed_3 (`self.LerpSetEmissiveFXValue` 0.0 (* (`self.EmissiveFXSpeed`) 0.5)))
                  (if _completed_3
                    (goto _label_3 :!via `Cancel`)))))))))))

(event `self.ReceiveBeginPlay`
  (bind _entrymontagestoplay (`self.EntryMontagesToPlay`))
  (bind _mesh (`self.Mesh`))
  (bind _outitem (`KismetArrayLibrary.Array_Random` _entrymontagestoplay))
  (`|ExecutionSequence`
    (:`then_0`
      ;[1 1 1] 敌人进场Montage动画和特效。
      (`TimelineComponent.SetPlayRate` (`self.EntryRestoreTimeline`) (/ 1.0 (`self.TotalEnteyRestoreTime`)))
      (bind (_direction _normalizedfloattrack) (`Timeline|EntryRestoreTimeline` :!via `ReverseFromEnd`)
        (:`Update`
          (`self.Set Dissolve` _normalizedfloattrack) ; 设置溶解效果。
        )))
    (:`then_1`
      (`AbilitySystemBlueprintLibrary.AddLooseGameplayTags` self (`BlueprintGameplayTagLibrary.MakeLiteralGameplayTagContainer` (struct :`GameplayTags` (struct :`(TagName` "Enemy.Status.Entering")))))
      (if (`KismetArrayLibrary.Array_IsNotEmpty` _entrymontagestoplay)
        (`|PlayMontage` (`self.Mesh`) _outitem
          (:`then`
            (`KismetSystemLibrary.Delay` (* (`AnimationAsset.GetPlayLength` _outitem) 0.5))))
        (else
          (`KismetSystemLibrary.Delay` 0.2)))
      (`WarriorFunctionLibrary.RemoveGameplayTagFromActorIfFound` self (struct :`TagName` "Enemy.Status.Entering")))
    (:`then_2`
      ;[1 1 1] 关闭物理布偶模拟。
      (`PrimitiveComponent.SetSimulatePhysics` _mesh false)
      (`PrimitiveComponent.SetCollisionProfileName` _mesh "CharacterMesh" true))))

(event `/Game/Gameplay/Characters/EnemyCharacter/BPI_EnemyDeath.OnEnemyDiedImmediately `
  ;[1 1 1] 死亡后立刻关闭人群避障组件。否则播放动画时的移动也会对其他角色的避障计算造成影响。比如死亡的小兵飞向Boss时，Boss为了避开会进行奇怪的转身行为。
  (`WarriorAIController.SetCrowdComponentDeactivate` (`self.WarriorAIController`)))

(event `/Game/Gameplay/Characters/EnemyCharacter/BPI_EnemyDeath.OnEnemyDiedAfterAnim`
  (params (DissolveNiagaraSystem :type "NiagaraSystem Soft Object Reference"))
  (bind _mesh (`self.Mesh`))
  (bind _mesh_2 (`self.Mesh`))
  (`|ExecutionSequence`
    (:`then_0`
      ;[1 1 1] 停止动画，关闭碰撞器。
      (set `SkeletalMeshComponent.bPauseAnims` true (`self.Mesh`))
      (`PrimitiveComponent.SetCollisionEnabled` (`self.CapsuleComponent`) "NoCollision")
      ;[1 1 1] 打开物理布偶模拟。
      (`PrimitiveComponent.SetCollisionProfileName` _mesh "Ragdoll" true)
      (`PrimitiveComponent.SetSimulatePhysics` _mesh true)
      ;;[1 1 1] 防止因动画导致物理骨骼陷入地里，在第一帧产生的极大力。
      (`WarriorFunctionLibrary.CountDown` 0.1 0.0
        (:`Update`
          (`PrimitiveComponent.SetAllPhysicsLinearVelocity` (`self.Mesh`) (0.0 0.0 1.0) false))))
    (:`then_1`
      ;[1 1 1] 移除敌人相关UI。
      (`EnemyUIComponent.RemoveEnemyDrawnWidgetsIfAny` (`self.EnemyUIComponent`)))
    (:`then_2`
      ;[1 1 1] 死亡特效FX。
      ;;[1 1 1] 创建并使用Niagara粒子特效。异步加载。
      (bind _object (`|LoadAsset` DissolveNiagaraSystem)
        (:`Completed`
          (bind _asniagara_system (cast `NiagaraSystem` _object))
          (bind _returnvalue (`NiagaraFunctionLibrary.SpawnSystemAttached` _asniagara_system (`self.Mesh`) "None" (0.0 0.0 0.0) (struct) "KeepRelativeOffset" true))
          ;;;[1 1 1] 将材质消融颜色给到粒子特效。保持视觉效果一致。
          (bind _returnvalue_2 (`PrimitiveComponent.CreateDynamicMaterialInstance` _mesh_2 0 (`PrimitiveComponent.GetMaterial` _mesh_2 0) "None"))
          (bind _returnvalue_3 (`MaterialInstanceDynamic.K2_GetVectorParameterValue` _returnvalue_2 "DissolveEdgeColor"))
          (`NiagaraComponent.SetNiagaraVariableLinearColor` _returnvalue "DissolveParticleColor" _returnvalue_3)
          ;;[1 1 1] 角色和武器消融效果。
          (`TimelineComponent.SetPlayRate` (`self.DissolveTimeline`) (/ 1.0 (`self.TotalDissolveTime`)))
          (bind (_direction _normalizedfloattrack) (`Timeline|DissolveTimeline` :!via `PlayFromStart`)
            (:`Update`
              (`self.Set Dissolve` _normalizedfloattrack) ; 设置溶解效果。
            )
            (:`Finished`
              (`self.OnDeathFXEnd`))))))))

(event `OnDeathFXEnd`
  (bind _returnvalue (`PawnCombatComponent.GetCharacterCurrentEquippedWeapon` (`self.EnemyCombatComponent`)))
  (`|ExecutionSequence`
    (:`then_0`
      (`|ExecutionSequence`
        (:`then_0`
          ;[1 1 1] 先销毁武器，因为我们需要通过角色Actor上的Combat组件获取当前武器。
          (`/Engine/EditorBlueprintResources/StandardMacros.IsValid` _returnvalue
            (:`Is Valid`
              (`self.K2_DestroyActor` _returnvalue))))
        (:`then_1`
          ;[1 1 1] 激活敌人掉落石头技能。
          (`WarriorAbilitySystemComponent.TryActivateAbilityByTag` (`self.WarriorAbilitySystemComponent`) (struct :`TagName` "Enemy.Ability.SpawnStone")))))
    (:`then_1`
      ;[1 1 1] 销毁自身角色。
      (`KismetSystemLibrary.Delay` 0.5) ; 为角色死亡技能生成石头等待。
      (`self.K2_DestroyActor`))))

(fn `LerpSetEmissiveFXColor`
  (params (TargetColor :type "LinearColor Structure" :default (struct :`R` 1.0 :`G` 1.0 :`B` 1.0 :`A` 1.0)) (Alpha :type "Float (single-precision)"))
  (returns (Completed :type Boolean))
  (locals (IsCompleted :type Boolean :default false))
  (`|ExecutionSequence`
    (:`then_0`
      (bind _output_get (set `self.EmissiveFXColorCurrent` (`KismetMathLibrary.LinearColorLerp` (`self.EmissiveFXColorCurrent`) TargetColor Alpha)))
      (bind _output_get_2 (set `local.IsCompleted` (`KismetMathLibrary.LinearColor_IsNearEqual` _output_get TargetColor)))
      (if _output_get_2
        (set `self.EmissiveFXColorCurrent` TargetColor)))
    (:`then_1`
      (`MeshComponent.SetVectorParameterValueOnMaterials` (`self.Mesh`) "HitEmissiveColor" (`KismetMathLibrary.Conv_LinearColorToVector` (`self.EmissiveFXColorCurrent`)))
      (return (`local.IsCompleted`)))))

(fn `LerpSetEmissiveFXValue`
  (params (Target :type "Float (double-precision)") (Alpha :type "Float (double-precision)" :default 0.1))
  (returns (Completed :type Boolean))
  (locals (IsCompleted :type Boolean :default false))
  (`|ExecutionSequence`
    (:`then_0`
      (bind _output_get (set `self.EmissiveFXValue` (`KismetMathLibrary.Lerp` (`self.EmissiveFXValue`) Target Alpha)))
      (bind _output_get_2 (set `local.IsCompleted` (`KismetMathLibrary.NearlyEqual_FloatFloat` _output_get Target)))
      (if _output_get_2
        (set `self.EmissiveFXValue` Target)))
    (:`then_1`
      (`MeshComponent.SetScalarParameterValueOnMaterials` (`self.Mesh`) "HitFxSwitch" (`self.EmissiveFXValue`))
      (return (`local.IsCompleted`)))))

(fn `Set Dissolve`
  (params (ParameterValue :type "Float (single-precision)"))
  (bind _returnvalue (`PawnCombatComponent.GetCharacterCurrentEquippedWeapon` (`self.EnemyCombatComponent`)))
  (`MeshComponent.SetScalarParameterValueOnMaterials` (`self.Mesh`) "DissolveAmount" ParameterValue)
  (`/Engine/EditorBlueprintResources/StandardMacros.IsValid` _returnvalue
    (:`Is Valid`
      (`MeshComponent.SetScalarParameterValueOnMaterials` (`WarriorWeaponBase.WeaponMesh` _returnvalue) "DissolveAmount" ParameterValue))))

(fn `UserConstructionScript`)