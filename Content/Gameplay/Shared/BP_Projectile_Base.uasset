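; Base projectile Blueprint that handles the sound and Niagara effects for spawning, flight and impact.
; On BeginPlay it plays a spawn sound, attaches a flight sound to the root component and spawns a muzzle effect facing the actor's forward vector.
; A separate OnSpawnProjectileHitFX event plays impact sound and effect at a supplied hit location.
; Each asset is validity-checked, and this graph contains no movement, collision or damage logic.
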(event `self.ReceiveBeginPlay`
  ;[1 1 1] 声音和Niagara特效。
  (`|ExecutionSequence`
    (:`then_0`
      (bind _projectilespawnsound (`self.ProjectileSpawnSound`)
        (:`then`
          (`GameplayStatics.PlaySoundAtLocation` _projectilespawnsound (`self.K2_GetActorLocation`) (struct) 1.0 1.0 0.0 null null null null))
        (:`else`)))
    (:`then_1`
      (bind _projectileflysound (`self.ProjectileFlySound`)
        (:`then`
          (`GameplayStatics.SpawnSoundAttached` _projectileflysound (`self.RootComponent`) "None" (0.0 0.0 0.0) (struct) "KeepRelativeOffset" true 1.0 1.0 0.0 null null) ; Stop when Attached to Destroyed = true
        )
        (:`else`)))
    (:`then_2`
      (bind _projectilemuzzlefx (`self.ProjectileMuzzleFX`)
        (:`then`
          (`NiagaraFunctionLibrary.SpawnSystemAtLocation` _projectilemuzzlefx (`self.K2_GetActorLocation`) (`KismetMathLibrary.Conv_VectorToRotator` (`self.GetActorForwardVector`))))
        (:`else`)))))

(event `self.BP_OnSpawnProjectileHitFX`
  (params (HitLocation :type "Vector Structure (by ref)"))
  ;[1 1 1] 播放炮弹击中声音和特效。
  (`|ExecutionSequence`
    (:`then_0`
      (bind _projectileimpactsound (`self.ProjectileImpactSound`)
        (:`then`
          (`GameplayStatics.PlaySoundAtLocation` _projectileimpactsound HitLocation (struct) 1.0 1.0 0.0 null null null null))
        (:`else`)))
    (:`then_1`
      (bind _projectileimpactfx (`self.ProjectileImpactFX`)
        (:`then`
          (`NiagaraFunctionLibrary.SpawnSystemAtLocation` _projectileimpactfx HitLocation))
        (:`else`)))))

(fn `UserConstructionScript`)